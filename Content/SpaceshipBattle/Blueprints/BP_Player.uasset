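; Player spaceship pawn that flies on world X/Y, aims at the mouse cursor and fires bullets.
; Tick consumes movement input as a swept offset, toggles thruster particles, and turns toward the cursor, deprojected at camera-to-ship distance and flattened to the ship's height.
; Held fire spawns BP_Bullet through a short Delay cooldown.
; Overlapping an enemy hides the ship, stops control, spawns a color-tinted Niagara explosion, then opens TutorialMap after a delay.
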(event OnComponentBeginOverlap(Collision)
  (params (OverlappedComponent :type Primitive%20Component%20Object%20Reference) (OtherActor :type Actor%20Object%20Reference) (OtherComp :type Primitive%20Component%20Object%20Reference) (OtherBodyIndex :type Integer) (bFromSweep :type Boolean) (SweepResult :type Hit%20Result%20Structure%20%28by%20ref%29))
  (Utilities|Casting|CastToBP_Enemy OtherActor)
  (CallFunction|OnDeath))

(event Custom|OnDeath
  (Utilities|FlowControl|Sequence
    (:then_0
      (Variables|Default|SetDead true)
      (Rendering|SetVisibility (Variables|Default|GetCollision) false true)
      (bind _returnvalue (Niagara|SpawnSystematLocation "/Game/SpaceshipBattle/ParticleSystems/PS_Explosion.PS_Explosion" (Transformation|GetActorLocation)))
      (Niagara|SetNiagaraVariable(LinearColor) _returnvalue "PrimaryColor" (Variables|Default|GetPrimaryColor))
      (Niagara|SetNiagaraVariable(LinearColor) _returnvalue "SecondaryColor" (Variables|Default|GetSecondaryColor))
      (Utilities|FlowControl|Delay 2.0)
      (Game|OpenLevel(byName) "TutorialMap"))))

(event EventBeginPlay
  (Variables|/Script/Engine.PlayerController|SetbShowMouseCursor (Game|GetPlayerController 0) true))

(event EventTick
  (params (DeltaSeconds :type Float%20%28single-precision%29))
  (CallFunction|Update))

(event Input|AxisEvents|InputAxisMoveUp
  (params (AxisValue :type Float%20%28single-precision%29))
  (Pawn|Input|AddMovementInput "1.000000,0.000000, 0" AxisValue false))

(event Input|AxisEvents|InputAxisMoveRight
  (params (AxisValue :type Float%20%28single-precision%29))
  (Pawn|Input|AddMovementInput "0.000000,1.000000, 0" AxisValue false))

(event Input|AxisEvents|InputAxisFire
  (params (AxisValue :type Float%20%28single-precision%29))
  (if (Math|Boolean|ANDBoolean (> AxisValue 0.0) (Variables|Default|GetCanShoot) (not (Variables|Default|GetDead)))
    (Game|SpawnActorfromClass "/Game/SpaceshipBattle/Blueprints/BP_Bullet.BP_Bullet_C" (Transformation|GetWorldTransform (Variables|Default|GetBulletSpawnPoint)) "Undefined" "OverrideRootScale" 0 0)
    (Variables|Default|SetCanShoot false)
    (Utilities|FlowControl|Delay 0.1)
    (Variables|Default|SetCanShoot true)))

(fn ConstructionScript)

(fn LookatCursor
  (bind _returnvalue (Transformation|GetActorLocation))
  (bind _returnvalue_2 (Game|GetPlayerController 0))
  (bind _camera (Variables|Default|GetCamera))
  (bind _shipmesh (Variables|Default|GetShipMesh))
  (bind _returnvalue_3 (Transformation|GetWorldLocation _camera))
  (bind _returnvalue_4 (Transformation|GetWorldLocation _shipmesh))
  (bind (_worldlocation _worlddirection) (Game|Player|ConvertMouseLocationToWorldSpace _returnvalue_2))
  (bind _returnvalue_5 (- _returnvalue_4 _returnvalue_3))
  (bind _returnvalue_6 (Math|Vector|VectorLength _returnvalue_5))
  (bind _returnvalue_7 (* _worlddirection _returnvalue_6))
  (bind _returnvalue_8 (+ _worldlocation _returnvalue_7))
  (bind (_x _y) (Math|Vector|BreakVector _returnvalue_8))
  (Transformation|SetActorRotation (Math|Rotator|FindLookatRotation _returnvalue (Math|Vector|MakeVector _x _y (.Z (Math|Vector|BreakVector _returnvalue))))))

(fn Move
  (bind _returnvalue (Class|Pawn|ConsumeMovementInputVector))
  (Transformation|AddActorWorldOffset (* _returnvalue (* (Utilities|Time|GetWorldDeltaSeconds) (Variables|Default|GetSpeed))) true))

(fn Update
  (if (not (Variables|Default|GetDead))
    (CallFunction|Move)
    (CallFunction|LookatCursor)
    (if (and (== (Input|AxisValues|GetMoveUp) 0.0) (== (Input|AxisValues|GetMoveRight) 0.0))
      (Components|Activation|Deactivate (Variables|Default|GetPS_Thruster))
      (else
        (Components|Activation|Activate (Variables|Default|GetPS_Thruster) false)))))